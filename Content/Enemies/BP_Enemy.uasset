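; Base enemy for turn-based combat that the player selects by click or touch, showing arrows on only that enemy.
; On BeginPlay it links itself to its health bar widget and creates a dynamic sprite material.
; EnemyTurn either clears a stun or randomly damages the player, shields a random enemy or heals a random enemy, with sound cues.
; TriggerFlash drives the material's flash through a timeline for stun and heal feedback.
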(event `self.ReceiveBeginPlay`
  (bind _asenemy_health_bar (cast `/Game/Enemies/Enemy_HealthBar` (`WidgetComponent.GetUserWidgetObject` (`self.HealthBar`))))
  (set `/Game/Enemies/Enemy_HealthBar.Enemy_Ref` self _asenemy_health_bar)
  (bind _returnvalue (`PrimitiveComponent.CreateDynamicMaterialInstance` (`self.Sprite`) 0 null "None"))
  (set `self.DynamicSpriteMat` _returnvalue))

(event `self.ReceiveActorOnInputTouchBegin`
  (params (FingerIndex :type "ETouchIndex Enum" :default "Touch1"))
  (bind _asplayer_pawn (cast `/Game/Player/PlayerPawn` (`GameplayStatics.GetPlayerPawn` 0) :!label _label))
  (set `/Game/Player/PlayerPawn.SelectedActor` self _asplayer_pawn)
  (bind _outactors (`GameplayStatics.GetAllActorsOfClass` "BP_Enemy_C"))
  (for _array_element _outactors
    (bind _output_get (set `/Game/Enemies/BP_Enemy.IsSelected` false _array_element))
    (`SceneComponent.SetVisibility` (`/Game/Enemies/BP_Enemy.SelectedArrows` _array_element) _output_get false)
    (bind _output_get_2 (set `self.IsSelected` true))
    (`SceneComponent.SetVisibility` (`self.SelectedArrows`) _output_get_2 false)))

(event `self.ReceiveActorOnClicked`
  (params (ButtonPressed :type "Key Structure"))
  (goto _label))

(event `EnemyTurn`
  (params (ButtonPressed :type "Key Structure"))
  (if (`self.IsStuned`)
    (`self.TriggerFlash` 1.0 (struct :`R` 1.0 :`G` 0.773535 :`A` 1.0))
    (set `self.IsStuned` false)
    (else
      (switch `int` (`KismetMathLibrary.RandomIntegerInRange` (`self.MinimumAction`) (`self.MaximumAction`))
        (:`0`
          (bind _asplayer_pawn (cast `/Game/Player/PlayerPawn` (`GameplayStatics.GetPlayerPawn` 0)))
          (set `/Game/Player/PlayerPawn.Health` (- (`/Game/Player/PlayerPawn.Health` _asplayer_pawn) (`self.Damage`)) _asplayer_pawn)
          (`GameplayStatics.PlaySound2D` "/Game/Sounds/Enemy_Attack_Cue.Enemy_Attack_Cue" 1.0 1.0 0.0 null null))
        (:`1`
          (bind _outactors (`GameplayStatics.GetAllActorsOfClass` "BP_Enemy_C"))
          (bind _outitem (`KismetArrayLibrary.Array_Random` _outactors))
          (bind _output_get (set `/Game/Enemies/BP_Enemy.IsProtected` true _outitem))
          (`SceneComponent.SetVisibility` (`/Game/Enemies/BP_Enemy.Shield` _outitem) _output_get true)
          (`GameplayStatics.PlaySound2D` "/Game/Sounds/Shield_Sound_Cue.Shield_Sound_Cue" 1.0 1.0 0.0 null null))
        (:`2`
          (bind _outactors_2 (`GameplayStatics.GetAllActorsOfClass` "BP_Enemy_C"))
          (bind _outitem_2 (`KismetArrayLibrary.Array_Random` _outactors_2))
          (bind _health (`/Game/Enemies/BP_Enemy.Health` _outitem_2))
          (set `/Game/Enemies/BP_Enemy.Health` (`KismetMathLibrary.FClamp` (+ _health (`self.HealValue`)) _health (`/Game/Enemies/BP_Enemy.MaxHealth` _outitem_2)) _outitem_2)
          (`GameplayStatics.PlaySound2D` "/Game/Sounds/Heal_Sound_Cue.Heal_Sound_Cue" 1.0 1.0 0.0 null null)
          (`self.TriggerFlash` 1.0 (struct :`G` 1.0 :`B` 0.091554 :`A` 1.0)))))))

(event `TriggerFlash`
  (params (Multiplier :type "Float (single-precision)" :default 1.0) (Color :type "LinearColor Structure" :default (struct :`R` 1.0 :`G` 0.012278 :`A` 1.0)) (PlayRate :type "Float (single-precision)" :default 5.0))
  (`MaterialInstanceDynamic.SetScalarParameterValue` (`self.DynamicSpriteMat`) "FlashMultiplier" Multiplier)
  (`MaterialInstanceDynamic.SetVectorParameterValue` (`self.DynamicSpriteMat`) "FlashColor" Color)
  (`TimelineComponent.SetPlayRate` (`self.FlashMultiplier`) PlayRate)
  (bind (_direction _alpha) (`Timeline|FlashMultiplier` :!via `PlayFromStart`)
    (:`Update`
      (`MaterialInstanceDynamic.SetScalarParameterValue` (`self.DynamicSpriteMat`) "FlashMultiplier" (`KismetMathLibrary.Lerp` 0.0 Multiplier _alpha)))))

(fn `UserConstructionScript`
  (set `self.Health` (`self.MaxHealth`)))